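; BP_Fruit is a sliceable fruit actor that launches upward on spawn, enables mouse interaction and destroys itself after a timeout.
; The construction script randomizes its material; coconut appears twice, pineapple never.
; After a short delay, cursor-over or click adds a point if the controller widget's Points is non-empty, then destroys it.
; Cursor-over also spawns a destroyed variant chosen by material display name, though the apple branch sets no class.
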(event OnBeginCursorOver(Plane)
  (params (TouchedComponent :type Primitive%20Component%20Object%20Reference))
  (bind _plane (Variables|Default|GetPlane))
  (bind _plane_2 (Variables|Default|GetPlane))
  (bind _plane_3 (Variables|Default|GetPlane))
  (bind _plane_4 (Variables|Default|GetPlane))
  (bind _plane_5 (Variables|Default|GetPlane))
  (bind _plane_6 (Variables|Default|GetPlane))
  (bind _returnvalue (Transformation|GetWorldLocation _plane))
  (bind _returnvalue_2 (Transformation|GetWorldLocation _plane_2))
  (bind _returnvalue_3 (Transformation|GetWorldLocation _plane_3))
  (bind _returnvalue_4 (Transformation|GetWorldLocation _plane_4))
  (bind _returnvalue_5 (Transformation|GetWorldLocation _plane_5))
  (bind _returnvalue_6 (Transformation|GetWorldLocation _plane_6))
  (Utilities|FlowControl|Delay 0.15)
  (if (> (Utilities|Array|Length (Variables|/Game/W_Drawing.W_Drawing_C|GetPoints (Variables|/Game/BP_PlayerControllerGame.BP_PlayerControllerGame_C|GetwidgetVariable (Variables|Default|GetAs%20BP%20Player%20Controller%20Game)))) 0)
    (Default|AddPoints (Variables|Default|GetAs%20BP%20Player%20Controller%20Game) 1)
    (if (Utilities|Enum|Equal(Enum) "apple_Mat" (Utilities|GetDisplayName (Rendering|Material|GetMaterial (Variables|Default|GetPlane) 0)))
      (Game|SpawnActorfromClass "/Game/BP_Destroyed_Apple.BP_Destroyed_Apple_C" (Math|Transform|MakeTransform (Math|Vector|MakeVector (.x _returnvalue) (.y _returnvalue) (.z _returnvalue)) "0, 0, 0" "2.000000,2.000000,2.000000") "Undefined" "MultiplyWithRoot" 0 0)
      (Actor|DestroyActor)
      (elif (Utilities|Enum|Equal(Enum) "banana_Mat" (Utilities|GetDisplayName (Rendering|Material|GetMaterial (Variables|Default|GetPlane) 0)))
        (Game|SpawnActorfromClass "/Game/BP_Destroyed_Banana.BP_Destroyed_Banana_C" (Math|Transform|MakeTransform (Math|Vector|MakeVector (.x _returnvalue_2) (.y _returnvalue_2) (.z _returnvalue_2)) "0, 0, 0" "2.000000,2.000000,2.000000") "Undefined" "MultiplyWithRoot" 0 0)
        (Actor|DestroyActor)
        (elif (Utilities|Enum|Equal(Enum) "coconut_Mat" (Utilities|GetDisplayName (Rendering|Material|GetMaterial (Variables|Default|GetPlane) 0)))
          (Game|SpawnActorfromClass "/Game/BP_Destroyed_Coconut.BP_Destroyed_Coconut_C" (Math|Transform|MakeTransform (Math|Vector|MakeVector (.x _returnvalue_3) (.y _returnvalue_3) (.z _returnvalue_3)) "0, 0, 0" "2.000000,2.000000,2.000000") "Undefined" "MultiplyWithRoot" 0 0)
          (Actor|DestroyActor)
          (elif (Utilities|Enum|Equal(Enum) "orange_Mat" (Utilities|GetDisplayName (Rendering|Material|GetMaterial (Variables|Default|GetPlane) 0)))
            (Game|SpawnActorfromClass "/Game/BP_Destroyed_Orange.BP_Destroyed_Orange_C" (Math|Transform|MakeTransform (Math|Vector|MakeVector (.x _returnvalue_4) (.y _returnvalue_4) (.z _returnvalue_4)) "0, 0, 0" "2.000000,2.000000,2.000000") "Undefined" "MultiplyWithRoot" 0 0)
            (Actor|DestroyActor)
            (elif (Utilities|Enum|Equal(Enum) "pineapple_Mat" (Utilities|GetDisplayName (Rendering|Material|GetMaterial (Variables|Default|GetPlane) 0)))
              (Game|SpawnActorfromClass "/Game/BP_Destroyed_Pineapple.BP_Destroyed_Pineapple_C" (Math|Transform|MakeTransform (Math|Vector|MakeVector (.x _returnvalue_5) (.y _returnvalue_5) (.z _returnvalue_5)) "0, 0, 0" "2.000000,2.000000,2.000000") "Undefined" "MultiplyWithRoot" 0 0)
              (Actor|DestroyActor)
              (else
                (Game|SpawnActorfromClass "/Game/BP_Destroyed_Watermelon.BP_Destroyed_Watermelon_C" (Math|Transform|MakeTransform (Math|Vector|MakeVector (.x _returnvalue_6) (.y _returnvalue_6) (.z _returnvalue_6)) "0, 0, 0" "2.000000,2.000000,2.000000") "Undefined" "MultiplyWithRoot" 0 0)
                (Actor|DestroyActor)))))))))

(event OnClicked(Plane)
  (params (TouchedComponent :type Primitive%20Component%20Object%20Reference) (ButtonPressed :type Key%20Structure :default "None"))
  (Utilities|FlowControl|Delay 0.15)
  (if (> (Utilities|Array|Length (Variables|/Game/W_Drawing.W_Drawing_C|GetPoints (Variables|/Game/BP_PlayerControllerGame.BP_PlayerControllerGame_C|GetwidgetVariable (Variables|Default|GetAs%20BP%20Player%20Controller%20Game)))) 0)
    (Default|AddPoints (Variables|Default|GetAs%20BP%20Player%20Controller%20Game) 1)
    (Actor|DestroyActor)))

(event EventBeginPlay
  (bind _returnvalue (Game|GetPlayerController 0))
  ;[1 1 1] Придаем ускоренние вверх
  (Physics|SetPhysicsLinearVelocity (Variables|Default|GetPlane) "0.000000,0.000000,1200.000000" false "None")
  (bind _asbp_player_controller_game (Utilities|Casting|CastToBP_PlayerControllerGame _returnvalue))
  (Variables|Default|SetAs%20BP%20Player%20Controller%20Game _asbp_player_controller_game)
  (Variables|/Script/Engine.PlayerController|SetbEnableMouseOverEvents _returnvalue true)
  (Variables|/Script/Engine.PlayerController|SetbEnableClickEvents _returnvalue true)
  (Variables|/Script/Engine.PlayerController|SetbShowMouseCursor _returnvalue true)
  (Utilities|FlowControl|Delay 9.0)
  (Actor|DestroyActor))

(fn ConstructionScript
  (bind _plane (Variables|Default|GetPlane))
  (switch int (Math|Random|RandomIntegerinRange 0 5)
    (:0
      (Rendering|Material|SetMaterial _plane 0 "/Game/img/apple_Mat.apple_Mat"))
    (:1
      (Rendering|Material|SetMaterial _plane 0 "/Game/img/banana_Mat.banana_Mat"))
    (:2
      (Rendering|Material|SetMaterial _plane 0 "/Game/img/coconut_Mat.coconut_Mat"))
    (:3
      (Rendering|Material|SetMaterial _plane 0 "/Game/img/coconut_Mat.coconut_Mat"))
    (:4
      (Rendering|Material|SetMaterial _plane 0 "/Game/img/orange_Mat.orange_Mat"))
    (:5
      (Rendering|Material|SetMaterial _plane 0 "/Game/img/watermelon_Mat.watermelon_Mat"))))